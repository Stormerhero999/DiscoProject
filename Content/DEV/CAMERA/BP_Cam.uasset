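; Two-player race camera that auto-scrolls along a spline, creates the HUD and declares a winner when the trailing player leaves view.
; After a one-second start delay, Tick eases the spring arm toward the next spline point, pushing X forward to the leader if ahead.
; Arm length zooms with player separation.
; An off-screen trailing player spawns the win widget for the leader every such frame; debug spheres and prints remain.
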(event Custom|SetupViewCamera
  (Game|Player|SetViewTargetwithBlend (Game|GetPlayerController 0) self 0.0 "VTBlend_Linear" 0.0 false)
  (Variables|Default|SetPlayers (Utilities|Array|MakeArray (Game|GetPlayerCharacter 0) (Game|GetPlayerCharacter 1))))

(event EventBeginPlay
  (bind _returnvalue (UserInterface|CreateWidget "/Game/DEV/UI/WBP_HUD.WBP_HUD_C"))
  (UserInterface|Viewport|AddtoViewport _returnvalue 0)
  (Utilities|FlowControl|Delay 1.0)
  (Variables|Default|SetStarting true))

(event EventTick
  (params (DeltaSeconds :type Float%20%28single-precision%29))
  (bind _springarm (Variables|Default|GetSpringArm))
  (bind _players (Variables|Default|GetPlayers))
  (bind _spline (Variables|Default|GetSpline))
  (bind _speed (Variables|Default|GetSpeed))
  (bind _returnvalue (Transformation|GetWorldLocation _springarm))
  (bind _output (Utilities|Array|Get(acopy) _players))
  (bind _output_2 (Utilities|Array|Get(acopy) _players 1))
  (bind _returnvalue_2 (* DeltaSeconds _speed 1e+03))
  (bind _returnvalue_3 (Class|SplineComponent|GetDistanceAlongSplineatLocation _spline _returnvalue "World"))
  (bind _returnvalue_4 (+ _returnvalue_3 _returnvalue_2))
  (bind _returnvalue_5 (Spline|GetLocationatDistanceAlongSpline _spline _returnvalue_4 "World"))
  (bind (_x _y _z) (Math|Vector|BreakVector _returnvalue_5))
  (if (Variables|Default|GetStarting)
    (bind _output_get (Variables|Default|SetPlayerAhead (select (<= (.X (Math|Vector|BreakVector (Transformation|GetActorLocation _output))) (.X (Math|Vector|BreakVector (Transformation|GetActorLocation _output_2)))) _output_2 _output)))
    (Variables|Default|SetTargetLocation (select (>= (.X (Math|Vector|BreakVector (Transformation|GetActorLocation _output_get))) _x) (Math|Vector|MakeVector (.X (Math|Vector|BreakVector (Transformation|GetActorLocation _output_get))) _y _z) (Math|Vector|MakeVector _x _y _z)))
    (Transformation|SetWorldLocation (Variables|Default|GetSpringArm) (Math|Interpolation|VInterpTo (Transformation|GetWorldLocation (Variables|Default|GetSpringArm)) (Variables|Default|GetTargetLocation) (Utilities|Time|GetWorldDeltaSeconds) 1e+01) false true)
    (Rendering|Debug|DrawDebugSphere (Variables|Default|GetTargetLocation) 1e+02 12 "(R=0.048799,G=1.000000,B=0.000000,A=1.000000)" 0.0 2.0)
    (Rendering|Debug|DrawDebugSphere (Math|Interpolation|VInterpTo (Transformation|GetWorldLocation (Variables|Default|GetSpringArm)) (Variables|Default|GetTargetLocation) (Utilities|Time|GetWorldDeltaSeconds) 1e+01) 1e+02 12 "(R=1.000000,G=0.310357,B=0.150163,A=1.000000)" 0.0 2.0)
    (CallFunction|CheckLastPlayerWasRecentlyRendered)
    (CallFunction|Zoom/DeZoom)))

(fn ConstructionScript)

(fn CheckLastPlayerWasRecentlyRendered
  (bind _players (Variables|Default|GetPlayers))
  (bind _output (Utilities|Array|Get(acopy) _players))
  (bind _output_2 (Utilities|Array|Get(acopy) _players 1))
  (if (Class|Actor|WasRecentlyRendered (select (< (.X (Math|Vector|BreakVector (Transformation|GetActorLocation _output_2))) (.X (Math|Vector|BreakVector (Transformation|GetActorLocation _output)))) _output_2 _output) 0.1)
    (Development|PrintString "proche cam" true true "(R=0.000000,G=0.660000,B=1.000000,A=1.000000)" 0.0)
    (else
      (Development|PrintString "loin cam" true true "(R=0.000000,G=0.660000,B=1.000000,A=1.000000)" 0.0)
      (bind _returnvalue (UserInterface|CreateWidget "/Game/DEV/UI/WBP_Win.WBP_Win_C"))
      (Default|WhoWin _returnvalue (Variables|Default|GetPlayerAhead))
      (UserInterface|Viewport|AddtoViewport _returnvalue 0))))

(fn Zoom/DeZoom
  (bind _players (Variables|Default|GetPlayers))
  (if (> (Transformation|GetDistanceTo (Utilities|Array|Get(acopy) _players) (Utilities|Array|Get(acopy) _players 1)) (Variables|Default|GetGapCheckBetween2%20Players))
    (Variables|/Script/Engine.SpringArmComponent|SetTargetArmLength (Variables|Default|GetSpringArm) (Math|Float|Clamp(Float) (+ (Variables|/Script/Engine.SpringArmComponent|GetTargetArmLength (Variables|Default|GetSpringArm)) (Variables|Default|GetSpeedZoom/Dezoom)) (Variables|Default|GetArmLengthMin) (Variables|Default|GetArmLengthMax)))
    (else
      (Variables|/Script/Engine.SpringArmComponent|SetTargetArmLength (Variables|Default|GetSpringArm) (Math|Float|Clamp(Float) (- (Variables|/Script/Engine.SpringArmComponent|GetTargetArmLength (Variables|Default|GetSpringArm)) (Variables|Default|GetSpeedZoom/Dezoom)) (Variables|Default|GetArmLengthMin) (Variables|Default|GetArmLengthMax))))))