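; Spline-based camera actor for two players that advances at a pace set by their movement.
; InteractAugmentSpeed plays a timeline moving the Camera component along the Spline over TimeToCompleteSeconds.
; Once Check arms Tick, the actor jumps each frame to the spline point at a one-frame distance: leading player's MaxWalkSpeed when either moves forward in X, otherwise CamSlow.
; Tick prints X for debugging; an interpolated closest-point move is left unconnected.
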(event Custom|Check
  (Variables|Default|SetChecked? true))

(event EventInteractAugmentSpeed
  ;[1 1 1] Déplacement de la caméra
  (Components|Timeline|SetPlayRate (Variables|Default|GetMoveCamera) (/ 1.0 (Variables|Default|GetTimeToComplete%28Seconds%29)))
  (bind _camera (Timeline|MoveCamera Play)
    (:Update
      (Transformation|SetRelativeLocation (Variables|Default|GetCamera) (Spline|GetLocationatDistanceAlongSpline (Variables|Default|GetSpline) (Math|Float|Lerp 0.0 (Spline|GetSplineLength (Variables|Default|GetSpline)) _camera) "Local") false false))))

(event EventTick
  (params (DeltaSeconds :type Float%20%28single-precision%29))
  (if (Variables|Default|GetChecked?)
    (if (or (> (.x (Transformation|GetVelocity (Game|Player|GetPlayerPawn 0))) 1e+02) (> (.x (Transformation|GetVelocity (Game|Player|GetPlayerPawn 1))) 1e+02))
      (if (> (.x (Transformation|GetActorLocation (Game|Player|GetPlayerPawn 0))) (.x (Transformation|GetActorLocation (Game|Player|GetPlayerPawn 1))))
        (Variables|Default|SetDistance (* (Variables|/Script/Engine.CharacterMovementComponent|GetMaxWalkSpeed (Variables|/Script/Engine.Character|GetCharacterMovement (.AsBP%20Player (Utilities|Casting|CastToBP_Player (Game|Player|GetPlayerPawn 0))))) DeltaSeconds))
        (Transformation|SetActorLocation (Math|Vector|MakeVector (.x (Spline|GetLocationatDistanceAlongSpline (Variables|Default|GetSpline) (Variables|Default|GetDistance) "World")) (.y (Spline|GetLocationatDistanceAlongSpline (Variables|Default|GetSpline) (Variables|Default|GetDistance) "World")) (.z (Spline|GetLocationatDistanceAlongSpline (Variables|Default|GetSpline) (Variables|Default|GetDistance) "World"))) false false)
        (Development|PrintString (Utilities|String|ToString(Float) (.x (Spline|GetLocationatDistanceAlongSpline (Variables|Default|GetSpline) (Variables|Default|GetDistance) "World"))) true true "(R=0.000000,G=0.660000,B=1.000000,A=1.000000)" 0.0)
        (else
          (Variables|Default|SetDistance (* (Variables|/Script/Engine.CharacterMovementComponent|GetMaxWalkSpeed (Variables|/Script/Engine.Character|GetCharacterMovement (.AsBP%20Player (Utilities|Casting|CastToBP_Player (Game|Player|GetPlayerPawn 1))))) DeltaSeconds))
          (Transformation|SetActorLocation (Math|Vector|MakeVector (.x (Spline|GetLocationatDistanceAlongSpline (Variables|Default|GetSpline) (Variables|Default|GetDistance) "World")) (.y (Spline|GetLocationatDistanceAlongSpline (Variables|Default|GetSpline) (Variables|Default|GetDistance) "World")) (.z (Spline|GetLocationatDistanceAlongSpline (Variables|Default|GetSpline) (Variables|Default|GetDistance) "World"))) false false)
          (Development|PrintString (Utilities|String|ToString(Float) (.x (Spline|GetLocationatDistanceAlongSpline (Variables|Default|GetSpline) (Variables|Default|GetDistance) "World"))) true true "(R=0.000000,G=0.660000,B=1.000000,A=1.000000)" 0.0)))
      (else
        (Variables|Default|SetDistance (* (Variables|Default|GetCamSlow) DeltaSeconds))
        (Transformation|SetActorLocation (Math|Vector|MakeVector (.x (Spline|GetLocationatDistanceAlongSpline (Variables|Default|GetSpline) (Variables|Default|GetDistance) "World")) (.y (Spline|GetLocationatDistanceAlongSpline (Variables|Default|GetSpline) (Variables|Default|GetDistance) "World")) (.z (Spline|GetLocationatDistanceAlongSpline (Variables|Default|GetSpline) (Variables|Default|GetDistance) "World"))) false false)
        (Development|PrintString (Utilities|String|ToString(Float) (.x (Spline|GetLocationatDistanceAlongSpline (Variables|Default|GetSpline) (Variables|Default|GetDistance) "World"))) true true "(R=0.000000,G=0.660000,B=1.000000,A=1.000000)" 0.0)))))

(fn ConstructionScript)