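; BP_ChildPlayerTheoTest is a developer test child of a player Blueprint that prototypes a timed charge for a stick ability.
; A looping one-second timer adds ProgressPerSecond to StickProgression and sets HaveStick when the value exactly equals 1.0.
; Tick prints the progression on screen for debugging.
; The IA_UseStick input checks HaveStick but performs no action yet.
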(event Custom|ProgressionbarWithTime
  (Variables|Default|SetStickProgression (+ (Variables|Default|GetStickProgression) (Variables|Default|GetProgress%20per%20second)))
  (if (== (Variables|Default|GetStickProgression) 1.0)
    (Variables|Default|SetHaveStick? true)))

(event Input|EnhancedActionEvents|EnhancedInputActionIA_UseStick
  (params (ActionValue :type Boolean) (ElapsedSeconds :type Float%20%28double-precision%29) (TriggeredSeconds :type Float%20%28double-precision%29) (InputAction :type Input%20Action%20Object%20Reference :default "/Game/DEV/Maxime/Input/Action/IA_UseStick.IA_UseStick"))
  (:Started
    (if (Variables|Default|GetHaveStick?)
      _)))

(event EventBeginPlay
  (|CallParentFunction)
  (Utilities|Time|SetTimerbyEvent (delegate Custom|ProgressionbarWithTime) 1.0 true))

(event EventTick
  (params (DeltaSeconds :type Float%20%28single-precision%29))
  (Development|PrintString (Utilities|String|ToString(Float) (Variables|Default|GetStickProgression)) true true "(R=0.000000,G=0.660000,B=1.000000,A=1.000000)" 0.0))

(fn ConstructionScript
  (|CallParentFunction))