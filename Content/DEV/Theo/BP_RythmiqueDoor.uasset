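; BP_RythmiqueDoor is a door that closes when the player enters its trigger box and slows a player who touches it.
; The box overlap, gated by an Open flag, plays the CloseDoor timeline, which moves the Cube's relative location, then reverses after a delay and resets the flag when finished.
; The Cube's own overlap calls HitSlow on the player's TheoCompenent.
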(event OnComponentBeginOverlap(Box)
  (params (OverlappedComponent :type Primitive%20Component%20Object%20Reference) (OtherActor :type Actor%20Object%20Reference) (OtherComp :type Primitive%20Component%20Object%20Reference) (OtherBodyIndex :type Integer) (bFromSweep :type Boolean) (SweepResult :type Hit%20Result%20Structure%20%28by%20ref%29))
  (Utilities|Casting|CastToBP_Player OtherActor)
  (if (Variables|Default|GetOpen?)
    (Variables|Default|SetRelative%20Location (Variables|/Script/Engine.SceneComponent|GetRelativeLocation (Variables|Default|GetCube)))
    (bind _close_track (Timeline|Close%20Door PlayFromStart)
      (:Update
        (Transformation|SetRelativeLocation (Variables|Default|GetCube) (* _close_track (- (Variables|Default|GetRelative%20Location) "0.000000,0.000000,100.000000")) false false)
        (Variables|Default|SetOpen? false)
        (Utilities|FlowControl|Delay 3.0)
        (Timeline|Close%20Door Reverse))
      (:Finished
        (Variables|Default|SetOpen? true)))))

(event OnComponentBeginOverlap(Cube)
  (params (OverlappedComponent :type Primitive%20Component%20Object%20Reference) (OtherActor :type Actor%20Object%20Reference) (OtherComp :type Primitive%20Component%20Object%20Reference) (OtherBodyIndex :type Integer) (bFromSweep :type Boolean) (SweepResult :type Hit%20Result%20Structure%20%28by%20ref%29))
  (bind _asbp_player (Utilities|Casting|CastToBP_Player OtherActor))
  (Default|HitSlow (Variables|/Game/DEV/Maxime/Blueprint/BP_Player.BP_Player_C|GetTheoCompenent _asbp_player) "NewEnumerator1"))

(fn ConstructionScript)