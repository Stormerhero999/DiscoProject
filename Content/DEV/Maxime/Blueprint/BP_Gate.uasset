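; BP_Gate is a gate that checks whether a passing BP_Player holds a required pose: Top, Down, Left or Right.
; When the player overlaps its Box, VerifingPosing compares the player's two action axis values to ranges selected by the gate's Posing setting.
; Each pose needs one axis near its extreme and the other near center.
; The result is only printed as a pass or fail debug message.
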(event OnComponentBeginOverlap(Box)
  (params (OverlappedComponent :type Primitive%20Component%20Object%20Reference) (OtherActor :type Actor%20Object%20Reference) (OtherComp :type Primitive%20Component%20Object%20Reference) (OtherBodyIndex :type Integer) (bFromSweep :type Boolean) (SweepResult :type Hit%20Result%20Structure%20%28by%20ref%29))
  (bind _asbp_player (Utilities|Casting|CastToBP_Player OtherActor))
  (bind _output_get (Variables|Default|SetAs%20BP%20Player _asbp_player))
  (if (CallFunction|VerifingPosing _output_get)
    (Development|PrintString "GG")
    (else
      (Development|PrintString "Slow"))))

(event EventBeginPlay)

(event Collision|EventActorBeginOverlap
  (params (OtherActor :type Actor%20Object%20Reference)))

(event EventTick
  (params (DeltaSeconds :type Float%20%28single-precision%29)))

(fn ConstructionScript)

(fn VerifingPosing
  (params (Target :type BP%20Player%20Object%20Reference))
  (bind _posing (Variables|Default|GetPosing))
  (bind _posing_2 (Variables|Default|GetPosing))
  (return (and (Math|Float|InRange(Float) (Variables|/Game/DEV/Maxime/Blueprint/BP_Player.BP_Player_C|GetAction%20Value%20X Target) (Utilities|Select :Index _posing_2 :NewEnumerator0 -0.2 :NewEnumerator1 -0.2 :NewEnumerator2 -1.0 :NewEnumerator3 0.8) (Utilities|Select :Index _posing_2 :NewEnumerator0 0.2 :NewEnumerator1 0.2 :NewEnumerator2 -0.8 :NewEnumerator3 1.0)) (Math|Float|InRange(Float) (Variables|/Game/DEV/Maxime/Blueprint/BP_Player.BP_Player_C|GetAction%20Value%20Y Target) (Utilities|Select :Index _posing :NewEnumerator0 0.8 :NewEnumerator1 -1.0 :NewEnumerator2 -0.2 :NewEnumerator3 -0.2) (Utilities|Select :Index _posing :NewEnumerator0 1.0 :NewEnumerator1 -0.8 :NewEnumerator2 0.2 :NewEnumerator3 0.2)))))