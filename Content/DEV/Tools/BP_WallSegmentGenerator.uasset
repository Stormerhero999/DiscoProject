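; BP_WallSegmentGenerator is a dev tool Blueprint that builds a wall segment variant from window, window frame and top meshes.
; Its Construction Script always calls Randomize, as the branch condition is fixed to true, so selections reroll on every construction run.
; Randomize rerolls only parts whose include flag is set, then GenerateWall applies all three indices through AssignStaticMesh, clamping each to its array bounds.
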(fn ConstructionScript
  (if true
    (Randomize|Randomize)
    (else
      (CallFunction|GenerateWall))))

(fn AssignStaticMesh
  (params (Index :type Integer) (Component :type Static%20Mesh%20Component%20Object%20Reference) (Array :type Array%20of%20Static%20Mesh%20Object%20References))
  (Components|StaticMesh|SetStaticMesh Component (Utilities|Array|Get(acopy) Array (Math|Integer|Clamp(Integer) Index 0 (Utilities|Array|LastIndex Array)))))

(fn Randomize
  (Utilities|FlowControl|Sequence
    (:then_0
      (if (Variables|Window|GetIncludeWindowInRandom)
        (Variables|Window|SetWindowIndex (Math|Random|RandomIntegerinRange 0 (Utilities|Array|LastIndex (Variables|Window|GetWindowMeshes))))))
    (:then_1
      (if (Variables|Frame|GetIncludeWindowFrameInRandom)
        (Variables|Frame|SetWindowFrameIndex (Math|Random|RandomIntegerinRange 0 (Utilities|Array|LastIndex (Variables|Frame|GetWindowFrameMeshes))))))
    (:then_2
      (if (Variables|Tampon|GetIncludeTopInRandom)
        (Variables|Tampon|SetWindowTopIndex (Math|Random|RandomIntegerinRange 0 (Utilities|Array|LastIndex (Variables|Tampon|GetWindowTopMeshes))))))
    (:then_3
      (Variables|Randomize|SetRandomized true)
      (CallFunction|GenerateWall))))

(fn GenerateWall
  (CallFunction|AssignStaticMesh (Variables|Window|GetWindowIndex) (Variables|Default|GetWindow) (Variables|Window|GetWindowMeshes))
  (CallFunction|AssignStaticMesh (Variables|Frame|GetWindowFrameIndex) (Variables|Default|GetWindowFrame) (Variables|Frame|GetWindowFrameMeshes))
  (CallFunction|AssignStaticMesh (Variables|Tampon|GetWindowTopIndex) (Variables|Default|GetTop) (Variables|Tampon|GetWindowTopMeshes)))