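; Game mode for a local multiplayer session that spawns the players and runs the pre-start countdown.
; BeginPlay adds a local player, possesses a BP_Player per local controller with indexed SKE and ANIM values, then sets up the BP_Cam view.
; It shows a transition widget, then the HUD and countdown widget after a delay.
; A looping timer decrements the count, then removes the countdown and flags players and camera as started, without clearing itself.
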(event Custom|TimerStart
  (bind _timer (Variables|Default|GetTimer))
  (Math|Integer|DecrementInt _timer
    (:%20%20
      (if (<= _timer 0)
        (Widget|RemovefromParent (Variables|Default|GetWidgetTimerRef))
        (for _array_element (Variables|Default|GetPlayers)
          (bind _asbp_player (Utilities|Casting|CastToBP_Player _array_element))
          (Variables|/Game/DEV/Maxime/Blueprint/BP_Player.BP_Player_C|SetTimer? _asbp_player true)
          (Variables|/Game/DEV/CAMERA/BP_Cam.BP_Cam_C|SetStarting (Variables|Default|GetCam_Ref) true))))))

(event EventBeginPlay
  (Utilities|FlowControl|Sequence
    (:then_0
      (Class|GameplayStatics|CreatePlayer -1)
      (for _index (range 0 (- (Class|GameplayStatics|GetNumLocalPlayerControllers) 1))
        (bind _returnvalue (Game|SpawnActorfromClass "/Game/DEV/Maxime/Blueprint/BP_Player.BP_Player_C" (Math|Transform|MakeTransform "0, 0, 0" "0.000000,90.000000,0.000000" "1.000000,1.000000,1.000000") "Undefined" "MultiplyWithRoot" 0 (Utilities|Array|Get(acopy) (Variables|Default|GetSKE) _index) (Utilities|Array|Get(acopy) (Variables|Default|GetANIM) _index) 0))
        (Pawn|Possess (Game|GetPlayerController _index) _returnvalue)
        (Utilities|Array|AddUnique (Variables|Default|GetPlayers) _returnvalue))
      (bind _returnvalue_2 (Actor|GetActorOfClass "/Game/DEV/CAMERA/BP_Cam.BP_Cam_C"))
      (bind _output_get (Variables|Default|SetCam_Ref _returnvalue_2))
      (Default|SetupViewCamera _output_get))
    (:then_1
      (bind _returnvalue_3 (UserInterface|CreateWidget "/Game/DEV/LevelTestNelson/Bp_GAMEsTARTtRANSITION.Bp_GAMEsTARTtRANSITION_C"))
      (UserInterface|Viewport|AddtoViewport _returnvalue_3 0)
      (Utilities|FlowControl|Delay 3.5)
      (bind _returnvalue_4 (UserInterface|CreateWidget "/Game/DEV/UI/InGame/WBP_HUD.WBP_HUD_C"))
      (UserInterface|Viewport|AddtoViewport _returnvalue_4 0)
      (bind _returnvalue_5 (UserInterface|CreateWidget "/Game/DEV/LevelTestNelson/Wb_BeginTimer.Wb_BeginTimer_C"))
      (bind _output_get_2 (Variables|Default|SetWidgetTimerRef _returnvalue_5))
      (UserInterface|Viewport|AddtoViewport _output_get_2 1)
      (Utilities|Time|SetTimerbyEvent (delegate Custom|TimerStart) 1.0 true))))

(fn ConstructionScript
  (|CallParentFunction))