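; Audio-reactive test Blueprint that plays a sound on BeginPlay and scales a cube to the music.
; Each playback-percent callback converts progress to seconds using the sound's duration, then samples normalized Constant-Q spectrum data for channel 0 from an Audio Synesthesia NRT asset.
; It loops over the bands, setting the same cube's world scale from each doubled value, so only the last band determines the final size.
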(event Custom|PlaybackChange
  (params (PlayingSoundWave :type Sound%20Wave%20Object%20Reference) (PlaybackPercent :type Float%20%28single-precision%29))
  (Variables|Default|SetPlayTime%20 (* PlaybackPercent (Variables|Default|GetDurationMusic)))
  (for _array_element (Class|ConstantQNRT|GetNormalizedChannelConstantQatTime (Variables|Default|GetConstantef) (Variables|Default|GetPlayTime%20))
    (Transformation|SetWorldScale3D (Variables|Default|GetCube) (* _array_element 2.0))))

(event EventBeginPlay
  (Audio|Components|Audio|SetSound (Variables|Default|GetAudio) (Variables|Default|GetNew%20Sound))
  (Variables|Default|SetDurationMusic (Variables|/Script/Engine.SoundBase|GetDuration (Variables|Default|GetNew%20Sound)))
  (EventDispatchers|BindEventtoOnAudioPlaybackPercent (Variables|Default|GetAudio) (delegate Custom|PlaybackChange))
  (Audio|Components|Audio|Play (Variables|Default|GetAudio) 0.0))

(fn ConstructionScript)