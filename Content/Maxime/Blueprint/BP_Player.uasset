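; BP_Player is an auto-running player character that constantly moves along its forward vector and jumps on Enhanced Input, with release ending the jump.
; The construction script copies its tuning variables for speed, jump hold, air control and jump height into the movement and jump settings.
; InteractAugmentSpeed applies a temporary speed boost through a retriggerable delay, then restores normal speed.
; An unconnected camera view-target call never runs.
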(event Input|EnhancedActionEvents|EnhancedInputActionIA_Jump
  (params (ActionValue :type Boolean) (ElapsedSeconds :type Float%20%28double-precision%29) (TriggeredSeconds :type Float%20%28double-precision%29) (InputAction :type Input%20Action%20Object%20Reference :default "/Game/Maxime/Input/Action/IA_Jump.IA_Jump"))
  (:Started
    (Character|Jump))
  (:Completed
    (Character|StopJumping)))

(event EventBeginPlay)

(event EventInteractAugmentSpeed
  (Variables|Stick|SetDurationStick (Variables|Stick|GetDurationStick))
  (Variables|/Script/Engine.CharacterMovementComponent|SetMaxWalkSpeed (Variables|Character|GetCharacterMovement) (Variables|Stick|GetStickSpeedMAX))
  (Development|PrintString "Hello")
  (Utilities|FlowControl|RetriggerableDelay (Variables|Stick|GetDurationStick))
  (Variables|/Script/Engine.CharacterMovementComponent|SetMaxWalkSpeed (Variables|Character|GetCharacterMovement) (Variables|Movement|GetMaxSpeed)))

(event EventTick
  (params (DeltaSeconds :type Float%20%28single-precision%29))
  (Pawn|Input|AddMovementInput (Transformation|GetActorForwardVector) 1.0 false))

(fn ConstructionScript
  (Variables|/Script/Engine.CharacterMovementComponent|SetMaxWalkSpeed (Variables|Character|GetCharacterMovement) (Variables|Movement|GetMaxSpeed))
  (Variables|Default|SetJumpMaxHoldTime (Variables|Movement|GetJumpMaxHold))
  (Variables|/Script/Engine.CharacterMovementComponent|SetAirControl (Variables|Character|GetCharacterMovement) (Variables|Movement|GetAirControl))
  (Variables|/Script/Engine.CharacterMovementComponent|SetJumpZVelocity (Variables|Character|GetCharacterMovement) (Variables|Movement|GetJumpHeight)))