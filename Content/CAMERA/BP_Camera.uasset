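; BP_Camera is an actor that moves its camera along a spline path when play begins.
; The MoveCamera timeline's play rate is the inverse of TimeToCompleteSeconds, so that variable controls the travel duration.
; Each timeline update maps the track value to a distance along the spline and sets the camera's relative location from that local-space point, leaving rotation untouched.
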(event EventBeginPlay
  (Components|Timeline|SetPlayRate (Variables|Default|GetMoveCamera) (/ 1.0 (Variables|Default|GetTimeToComplete%28Seconds%29)))
  (bind _camera (Timeline|MoveCamera Play)
    (:Update
      (Transformation|SetRelativeLocation (Variables|Default|GetCamera) (Spline|GetLocationatDistanceAlongSpline (Variables|Default|GetSpline) (Math|Float|Lerp 0.0 (Spline|GetSplineLength (Variables|Default|GetSpline)) _camera) "Local") false false))))

(fn ConstructionScript)